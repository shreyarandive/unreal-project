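; HealthPickup is a pickup actor that restores a fixed amount of the player's health when overlapped.
; Any actor overlap calls AddHealth, which casts player character 0 to ThirdPersonCharacter without checking the overlapping actor.
; If Health is below 100, it adds the amount without clamping and toggles the root's visibility, propagating to children.
; The actor is never destroyed or disabled, so later overlaps can heal and toggle again.
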(event `self.ReceiveActorBeginOverlap`
  (params (OtherActor :type "Actor Object Reference"))
  (`self.AddHealth`))

(fn `AddHealth`
  (bind _asthird_person_character (cast `/Game/ThirdPersonBP/Blueprints/ThirdPersonCharacter` (`GameplayStatics.GetPlayerCharacter` 0)))
  (bind _health (`/Game/ThirdPersonBP/Blueprints/ThirdPersonCharacter.Health` _asthird_person_character))
  (if (< _health 100)
    (set `/Game/ThirdPersonBP/Blueprints/ThirdPersonCharacter.Health` (+ _health 10) _asthird_person_character)
    (`SceneComponent.ToggleVisibility` (`self.DefaultSceneRoot`) true)))

(fn `UserConstructionScript`)