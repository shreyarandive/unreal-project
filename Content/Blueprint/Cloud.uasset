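; Cloud actor that drifts its Cloud1 component back and forth along its relative Y axis.
; Each tick it sets the CloudMove offset to positive Y below a lower bound or negative Y above an upper bound, keeping the last value in between.
; It then adds that offset without sweeping; the fixed step ignores delta time, so speed depends on frame rate.
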(event `self.ReceiveTick`
  (params (DeltaSeconds :type "Float (single-precision)"))
  (bind _y (.y (.location (`SceneComponent.GetRelativeTransform` (`self.Cloud1`)))))
  (if (< _y 1000.0)
    (set `self.CloudMove` (0.0 5.0 0.0))
    (elif (> _y 6000.0)
      (set `self.CloudMove` (0.0 -5.0 0.0))))
  (`SceneComponent.K2_AddRelativeLocation` (`self.Cloud1`) (`self.CloudMove`) false false))

(fn `UserConstructionScript`)